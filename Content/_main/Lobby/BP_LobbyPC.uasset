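; Lobby player controller that creates and manages the lobby menu and loading screen widgets.
; InitialSetup, on authority, builds the menu with mouse input, then after short delays pushes map info to it and calls CallUpdate with player settings.
; ShowLoadingScreen replaces the menu with a loading widget, and T toggles menu and cursor visibility on authority.
; CallUpdate and SaveGame are empty stubs in this graph.
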(event `Initial Setup`
  (params (ServerName :type Text) (MapImage :type "Texture2D Object Reference") (MapName :type Text) (MapTime :type Text))
  (`/Engine/EditorBlueprintResources/ActorMacros.Switch Has Authority`
    (:`Authority`
      (`self.SetupLobbyMenu` ServerName)
      (`KismetSystemLibrary.Delay` 0.2)
      (`self.UpdateLobbySettings` MapImage MapName MapTime)
      (`KismetSystemLibrary.Delay` 0.2)
      (`self.CallUpdate` (`self.PlayerSettings`)))))

(event `SetupLobbyMenu`
  (params (ServerName :type Text))
  (set `self.bShowMouseCursor` true)
  (bind _returnvalue (`|CreateWidget` "/Game/_main/Lobby/LobbyMenu.LobbyMenu_C"))
  (bind _output_get (set `self.LobbyWidget` _returnvalue))
  (`UserWidget.AddToViewport` _output_get 0)
  (`WidgetBlueprintLibrary.SetInputMode_GameAndUIEx` self (`self.LobbyWidget`)))

(event `UpdateLobbySettings`
  (params (MapImage :type "Texture2D Object Reference") (MapName :type Text) (MapTime :type Text))
  (`/Game/_main/Lobby/LobbyMenu.UpdateLobbyInfo` (`self.LobbyWidget`) MapImage MapName MapTime))

(event `CallUpdate`
  (params (PlayerSettings :type "/Game/_main/S_PlayerInfo Structure") (`changedStatus?` :type Boolean)))

(event `ShowLoadingScreen`
  (`Widget.RemoveFromParent` (`self.LobbyWidget`))
  (bind _returnvalue (`|CreateWidget` "/Game/Widgets/LoadingScreen.LoadingScreen_C" self))
  (`UserWidget.AddToViewport` _returnvalue 0))

(event `Key|T`
  (params (Key :type "Key Structure"))
  (bind _lobbywidget (`self.LobbyWidget`))
  (:`Pressed`
    (`/Engine/EditorBlueprintResources/ActorMacros.Switch Has Authority`
      (:`Authority`
        (`/Engine/EditorBlueprintResources/StandardMacros.FlipFlop`
          (:`A`
            (`Widget.SetVisibility` _lobbywidget "Hidden")
            (set `self.bShowMouseCursor` false))
          (:`B`
            (`Widget.SetVisibility` _lobbywidget "Visible")
            (set `self.bShowMouseCursor` true)))))))

(event `SaveGame`)

(fn `LobbyPCRef`
  (returns (LobbyPc :type "/Game/_main/Lobby/BP_LobbyPC Object Reference"))
  (return null))

(fn `UserConstructionScript`)