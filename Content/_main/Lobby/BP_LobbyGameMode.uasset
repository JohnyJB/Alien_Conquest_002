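; Lobby game mode that registers joining players and launches the match from the lobby.
; On PostLogin it stores the player and PlayerStarts, reads server name and player limit from the Steam game instance, then sends lobby and map details to that player's controller.
; StartLoadingScreen shows each player's loading screen, then server-travels to the hard-coded FirstPersonExampleMap.
; SpawnPlayer is empty, and its call and the lobby-settings update are unwired.
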(event `self.K2_PostLogin`
  (params (NewPlayer :type "PlayerController Object Reference"))
  (bind _output_get (set `self.ConnectedPlayer` NewPlayer))
  (`KismetArrayLibrary.Array_AddUnique` (`self.Players`) _output_get)
  (bind _outactors (`GameplayStatics.GetAllActorsOfClass` "/Script/Engine.PlayerStart"))
  (set `self.SpawnPoints` _outactors)
  (bind _gameinstance (message `/Game/_main/BPI_GameInstance.SteamGameInstanceRef` (`GameplayStatics.GetGameInstance`)))
  (set `self.Server Name` (`/Game/_main/SteamGameInstance.ServerName` _gameinstance))
  (set `self.Max Players` (`/Game/_main/SteamGameInstance.MaxPlayers` _gameinstance))
  (bind _lobbypc (message `/Game/_main/Lobby/BPI_LobbyPC.LobbyPCRef` (`self.ConnectedPlayer`)))
  (`/Game/_main/Lobby/BP_LobbyPC.Initial Setup` _lobbypc (`self.Server Name`) (`self.SelectedMapImage`) (`self.SelectedMapName`) (`self.SelectedMapTime`)))

(event `SpawnPlayer`
  (params (Player :type "PlayerController Object Reference")))

(event `StartLoadingScreen`
  (for _array_element (`self.Players`)
    (bind _lobbypc (message `/Game/_main/Lobby/BPI_LobbyPC.LobbyPCRef` _array_element))
    (`/Game/_main/Lobby/BP_LobbyPC.ShowLoadingScreen` _lobbypc))
  (`self.LaunchGame`))

(event `LaunchGame`
  (`KismetSystemLibrary.ExecuteConsoleCommand` "servertravel/FirstPersonBP/Maps/FirstPersonExampleMap" (`GameplayStatics.GetPlayerController` 0)))

(fn `UserConstructionScript`)